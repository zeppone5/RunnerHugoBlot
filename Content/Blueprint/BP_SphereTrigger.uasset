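; BP_SphereTrigger is a trigger actor that keeps track of which BP_Coins actors are currently overlapping it.
; On BeginPlay it casts the game mode to GameModeRunner and caches the reference.
; Overlap begin and end events add each coin to, or remove it from, the game mode's Coins array, which therefore reflects the coins inside the trigger.
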(event EventBeginPlay
  (bind _asgame_mode_runner (Utilities|Casting|CastToGameModeRunner (Game|GetGameMode)))
  (Variables|Default|SetAs%20Game%20Mode%20Runner _asgame_mode_runner))

(event Collision|EventActorBeginOverlap
  (params (OtherActor :type Actor%20Object%20Reference))
  (bind _asbp_coins (Utilities|Casting|CastToBP_Coins OtherActor))
  (Utilities|Array|Add (Variables|/Script/Runner.GameModeRunner|GetCoins (Variables|Default|GetAs%20Game%20Mode%20Runner)) _asbp_coins))

(event Collision|EventActorEndOverlap
  (params (OtherActor :type Actor%20Object%20Reference))
  (bind _asbp_coins (Utilities|Casting|CastToBP_Coins OtherActor))
  (Utilities|Array|RemoveItem (Variables|/Script/Runner.GameModeRunner|GetCoins (Variables|Default|GetAs%20Game%20Mode%20Runner)) _asbp_coins))

(fn ConstructionScript)